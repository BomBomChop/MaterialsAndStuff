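; BP_DissolveShape is a placeable box volume that defines the shape used by dissolve materials.
; Its construction script writes the Cube component's world location, scale and forward, right and up vectors into the MPC_ShapeData parameter collection, giving materials an oriented box.
; The event graph is empty, so the blueprint has no runtime update, and every instance writes to the same shared parameters.
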(fn `UserConstructionScript`
  (`KismetMaterialLibrary.SetVectorParameterValue` "/Game/AdvancedMaterial/DissolveMaterial/ParamCollection/MPC_ShapeData.MPC_ShapeData" "Location" (`KismetMathLibrary.Conv_VectorToLinearColor` (`SceneComponent.K2_GetComponentLocation` (`self.Cube`))))
  (`KismetMaterialLibrary.SetVectorParameterValue` "/Game/AdvancedMaterial/DissolveMaterial/ParamCollection/MPC_ShapeData.MPC_ShapeData" "Bounds" (`KismetMathLibrary.Conv_VectorToLinearColor` (`SceneComponent.K2_GetComponentScale` (`self.Cube`))))
  (`KismetMaterialLibrary.SetVectorParameterValue` "/Game/AdvancedMaterial/DissolveMaterial/ParamCollection/MPC_ShapeData.MPC_ShapeData" "X" (`KismetMathLibrary.Conv_VectorToLinearColor` (`SceneComponent.GetForwardVector` (`self.Cube`))))
  (`KismetMaterialLibrary.SetVectorParameterValue` "/Game/AdvancedMaterial/DissolveMaterial/ParamCollection/MPC_ShapeData.MPC_ShapeData" "Y" (`KismetMathLibrary.Conv_VectorToLinearColor` (`SceneComponent.GetRightVector` (`self.Cube`))))
  (`KismetMaterialLibrary.SetVectorParameterValue` "/Game/AdvancedMaterial/DissolveMaterial/ParamCollection/MPC_ShapeData.MPC_ShapeData" "Z" (`KismetMathLibrary.Conv_VectorToLinearColor` (`SceneComponent.GetUpVector` (`self.Cube`)))))